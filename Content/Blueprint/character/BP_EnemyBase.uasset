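; Base enemy Blueprint handling spawn scale-in, dissolve effects, motion-warp facing and loot drops.
; BeginPlay scales the mesh via timeline; other timelines drive the Dissolve parameter on body and weapon materials.
; SpawnLoot rolls items from loot tiers, then a looping timer spawns them one by one around the enemy, passing Level to AuraEffectActors.
; GetLootTransform picks random distances along evenly spaced rotations and line-traces vertically to ground each drop.
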(event Custom|SpawnLootItem
  (bind _spawnloopcount (Variables|Default|GetSpawnLoopCount))
  (bind _lootitems (Variables|Default|GetLootItems))
  (bind _spawnloopcount_2 (Variables|Default|GetSpawnLoopCount))
  (bind _spawntransform (CallFunction|GetLootTransform _spawnloopcount))
  (bind _output (Utilities|Array|Get(acopy) _lootitems _spawnloopcount_2))
  (bind _lootclass (Utilities|Struct|BreakLootItem _output))
  (if (< (Variables|Default|GetSpawnLoopCount) (Utilities|Array|Length (Variables|Default|GetLootItems)))
    (bind _asaura_effect_actor (Utilities|Casting|CastToAuraEffectActorClass _lootclass)
      (:then
        (Game|SpawnActorfromClass _asaura_effect_actor _spawntransform "Undefined" "MultiplyWithRoot" 0 (Math|Conversions|ToFloat(Integer) (Variables|Default|GetLevel)) 0))
      (:CastFailed
        (Game|SpawnActorfromClass _lootclass _spawntransform "Undefined" "MultiplyWithRoot" 0 0)))
    (Math|Integer|IncrementInt (Variables|Default|GetSpawnLoopCount))
    (else
      (Utilities|Time|ClearandInvalidateTimerbyHandle (Variables|Default|GetLootTimer)))))

(event EventBeginPlay
  (bind _newtrack_0 (Timeline|SpawnTimeLine Play)
    (:Update
      (Transformation|SetRelativeScale3D (Variables|Character|GetMesh) (Math|Vector|MakeVector _newtrack_0 _newtrack_0 _newtrack_0)))))

(event Collision|EventActorBeginOverlap
  (params (OtherActor :type Actor%20Object%20Reference)))

(event EventTick
  (params (DeltaSeconds :type Float%20%28single-precision%29)))

(event EventStartDissolveTimeLine
  (params (DynamicMaterialInstance :type Material%20Instance%20Dynamic%20Object%20Reference))
  (bind _newtrack_0 (Timeline|DissolveTimeLine Play)
    (:Update
      (Rendering|Material|SetScalarParameterValue DynamicMaterialInstance "Dissolve" _newtrack_0 :!class /Script/Engine.MaterialInstanceDynamic))))

(event EventStartWeaponDissolveTimeLine
  (params (DynamicMaterialInstance :type Material%20Instance%20Dynamic%20Object%20Reference))
  (bind _newtrack_0 (Timeline|DissolveWeaponTimeLine Play)
    (:Update
      (Rendering|Material|SetScalarParameterValue DynamicMaterialInstance "Dissolve" _newtrack_0 :!class /Script/Engine.MaterialInstanceDynamic))))

(event EventUpdateFacingTarget
  (params (Target :type Vector%20%28by%20ref%29 :default "0, 0, 0"))
  (Class|MotionWarpingComponent|AddorUpdateWarpTargetfromLocation (Variables|Default|GetMotionWarping) "FacingTarget" Target))

(event EventSpawnLoot
  (bind _returnvalue (Class|AuraAbilitySystemLibrary|GetLootTiers))
  (Utilities|IsValid _returnvalue
    (:Is%20Valid
      (bind _returnvalue_2 (Class|LootTiers|GetLootItem _returnvalue))
      (bind _output_get (Variables|Default|SetLootItems _returnvalue_2))
      (bind _returnvalue_3 (Class|AuraAbilitySystemLibrary|EvenlySpacedRotators (Transformation|GetActorForwardVector) (Math|Vector|VectorUp) 3.6e+02 (Utilities|Array|Length _output_get)))
      (Variables|Default|SetLoootRotations _returnvalue_3)
      (Variables|Default|SetSpawnLoopCount 0)
      (bind _returnvalue_4 (Utilities|Time|SetTimerbyEvent (delegate Custom|SpawnLootItem) 0.1 true))
      (Variables|Default|SetLootTimer _returnvalue_4)
      (CallFunction|SpawnLootItem))))

(fn ConstructionScript)

(fn GetLootTransform
  (params (LoopCount :type Integer))
  (bind _returnvalue (Transformation|GetActorLocation))
  (bind _minspawndistance (Variables|Default|GetMinSpawnDistance))
  (bind _maxspawndistance (Variables|Default|GetMaxSpawnDistance))
  (bind _loootrotations (Variables|Default|GetLoootRotations))
  (bind _returnvalue_2 (Math|Random|RandomFloatinRange _minspawndistance _maxspawndistance))
  (bind _output (Utilities|Array|Get(acopy) _loootrotations LoopCount))
  (bind _returnvalue_3 (Math|Vector|GetForwardVector _output))
  (bind _returnvalue_4 (* _returnvalue_3 _returnvalue_2))
  (bind _returnvalue_5 (+ _returnvalue_4 _returnvalue))
  (bind _returnvalue_6 (Math|Transform|MakeTransform _returnvalue_5 _output))
  (bind (_x _y _z) (Math|Vector|BreakVector (.location _returnvalue_6)))
  (bind (_x_2 _y_2 _z_2) (Math|Vector|BreakVector (.location _returnvalue_6)))
  ;[1 1 1] 根据获取的旋转信息叠加敌人的位置，并拥有一定的位移
  (bind (_outhit _returnvalue_7) (Collision|LineTraceByChannel (Math|Vector|MakeVector _x_2 _y_2 (+ _z_2 5e+02)) (Math|Vector|MakeVector _x _y (+ _z -5e+02)) "TraceTypeQuery1" false 0 "None"))
  (if _returnvalue_7
    (return (Math|Transform|MakeTransform (.ImpactPoint (Collision|BreakHitResult _outhit)) (.rotation _returnvalue_6)))
    (else
      (return (Math|Transform|MakeTransform (.location _returnvalue_6) (.rotation _returnvalue_6) (.scale _returnvalue_6))))))