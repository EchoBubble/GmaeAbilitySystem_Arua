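; Fire Blast ability fireball that flies straight out along its forward vector, then returns to its ReturnToActor and explodes.
; On authority, an outgoing timeline lerps it to an apex point at TravelDistance.
; When that finishes, it empties its ignore list and a returning timeline lerps it toward the actor's live location.
; Once within ExplodeDistance of that actor, it calls OnHit and destroys itself.
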(event EventBeginPlay)

(event Collision|EventActorBeginOverlap
  (params (OtherActor :type Actor%20Object%20Reference)))

(event EventTick
  (params (DeltaSeconds :type Float%20%28single-precision%29)))

(event EventStartOutgoingTimeline
  (Networking|SwitchHasAuthority
    (:Authority
      ;[1 1 1] 储存最开始位置和最终位置
      (Variables|Default|SetInitialLocation (Transformation|GetActorLocation))
      (Variables|Default|SetApexLocation (+ (Variables|Default|GetInitialLocation) (* (Transformation|GetActorForwardVector) (Variables|Default|GetTravelDistance))))
      (bind _newtrack_0 (Timeline|OutgoingTimeline Play)
        (:Update
          (Transformation|SetActorLocation (Math|Vector|Lerp(Vector) (Variables|Default|GetInitialLocation) (Variables|Default|GetApexLocation) _newtrack_0) false false))
        (:Finished
          (Class|AuraFireBall|EmptyIgnoreList)
          (bind _newtrack_0_2 (Timeline|ReturningTimeline PlayFromStart)
            (:Update
              (Transformation|SetActorLocation (Math|Vector|Lerp(Vector) (Variables|Default|GetApexLocation) (Transformation|GetActorLocation (Variables|Default|GetReturnToActor)) _newtrack_0_2) false false)
              (if (CallFunction|IsWithinExplodeDistance)
                (Class|AuraProjectile|OnHit)
                (Actor|DestroyActor)))))))))

(fn ConstructionScript)

(fn IsWithinExplodeDistance
  (return (<= (Math|Vector|VectorLength (- (Transformation|GetActorLocation) (Transformation|GetActorLocation (Variables|Default|GetReturnToActor)))) (Variables|Default|GetExplodeDistance))))