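; BP_Aura_MainMenu sets up the main menu, with a Niagara effect that bobs up and down in the scene.
; On BeginPlay it creates WBP_MainMenu, adds it to the viewport, shows the cursor and switches input to UI only.
; A fast looping timer, rather than Tick, advances a wrapping time value that drives a sine offset on the effect's height around its starting position.
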(event Custom|CustomEvent
  (Variables|Default|SetTime (+ (Variables|Default|GetTime) 0.01))
  (if (> (Variables|Default|GetTime) 6.28)
    (Variables|Default|SetTime 0.0)
    (else
      (Transformation|SetWorldLocation (Variables|Default|GetNiagara) (+ (Variables|Default|GetFireBallLocation) (Math|Vector|MakeVector 0.0 0.0 (* (Math|Trig|Sin(Radians) (Variables|Default|GetTime)) (Variables|Default|GetAmplitude)))) false false))))

(event EventBeginPlay
  (bind _returnvalue (Game|GetPlayerController 0))
  (Variables|Default|SetFireBallLocation (Transformation|GetWorldLocation (Variables|Default|GetNiagara)))
  (bind _returnvalue_2 (Utilities|Time|SetTimerbyEvent (delegate Custom|CustomEvent) 0.01 true))
  (Variables|Default|SetTimer _returnvalue_2)
  (Utilities|IsValid _returnvalue
    (:Is%20Valid
      (bind _returnvalue_3 (UserInterface|CreateWidget "/Game/Blueprint/UI/MainManu/WBP_MainMenu.WBP_MainMenu_C" _returnvalue))
      (Input|SetInputModeUIOnly _returnvalue _returnvalue_3 "DoNotLock" false)
      (UserInterface|Viewport|AddtoViewport _returnvalue_3 0)
      (Variables|/Script/Engine.PlayerController|SetbShowMouseCursor _returnvalue true))))

(fn ConstructionScript)