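; BP_Pickup_Base is a base pickup actor that animates its appearance when play begins.
; A timeline raises it from its initial location by a spawn apex and drives its uniform scale.
; When the timeline finishes, it calls functions to start sinusoidal movement and rotation, whose bodies are not in this graph.
; Tick applies the calculated location and rotation to the actor every frame.
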(event EventBeginPlay
  (bind _initiallocation (Variables|Default|GetInitialLocation))
  (bind (_direction _elevation _scale) (Timeline|PickupElevation Play)
    (:Update
      (Variables|Default|SetCalculatedLocation (Math|Vector|MakeVector (.x _initiallocation) (.y _initiallocation) (+ (.z _initiallocation) (* _elevation (Variables|Default|GetSpawnApex)))))
      (Transformation|SetActorScale3D (Math|Vector|MakeVector _scale _scale _scale)))
    (:Finished
      (Class|AuraEffectActor|StartSinusoidalMovement)
      (Class|AuraEffectActor|StartRotation))))

(event Collision|EventActorBeginOverlap
  (params (OtherActor :type Actor%20Object%20Reference)))

(event EventTick
  (params (DeltaSeconds :type Float%20%28single-precision%29))
  (Transformation|SetActorLocation (Variables|Default|GetCalculatedLocation) false false)
  (Transformation|SetActorRotation (Variables|Default|GetCalculatedRotation)))

(fn ConstructionScript)